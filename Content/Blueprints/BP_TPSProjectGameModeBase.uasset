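; BP_TPSProjectGameModeBase is a game mode Blueprint that puts a score display on screen.
; On BeginPlay it creates a BP_Widget, stores it as WidgetTarget, adds it to the viewport and initializes its text.
; Every Tick, while that widget is valid, it rewrites the text as a score label built from HitCount, which is not modified in these graphs.
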(event EventBeginPlay
  (bind _returnvalue (UserInterface|CreateWidget "/Game/Blueprints/BP_Widget.BP_Widget_C"))
  (bind _output_get (Variables|Default|SetWidgetTarget _returnvalue))
  (UserInterface|Viewport|AddtoViewport _output_get 0)
  (Variables|/Game/Blueprints/BP_Widget.BP_Widget_C|SetTextVal _output_get "0"))

(event EventTick
  (params (DeltaSeconds :type Float%20%28single-precision%29))
  (bind _widgettarget (Variables|Default|GetWidgetTarget))
  (if (Utilities|IsValid _widgettarget)
    (Variables|/Game/Blueprints/BP_Widget.BP_Widget_C|SetTextVal _widgettarget (Utilities|String|Append "Score : " (Utilities|String|ToString(Integer) (Variables|Default|GetHitCount))))))

(fn ConstructionScript)